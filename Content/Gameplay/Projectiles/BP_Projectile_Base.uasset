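; Base projectile actor that deals damage to whatever it hits and then destroys itself.
; ProjectileName drives BPCProjectileStats configuration in the construction script, repeated at BeginPlay if unconfigured, setting movement speeds and gravity scale from those stats.
; Hits apply the stats' damage, crediting OwningWeapon as causer.
; The stats' damage type is read but unused, as BP_Damage_Base is always passed.
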(event EventBeginPlay
  (if (not (Variables|/Game/Gameplay/Components/BPC_Projectile_Stats.BPC_Projectile_Stats_C|GetIsConfigured (Variables|Default|GetBPC_Projectile_Stats)))
    (Config|ConfigureProjectileStatsComponent)
    (Config|SetProjectileParameters)))

(event Collision|EventActorBeginOverlap
  (params (OtherActor :type Actor%20Object%20Reference)))

(event EventTick
  (params (DeltaSeconds :type Float%20%28single-precision%29)))

(event Collision|EventHit
  (params (MyComp :type Primitive%20Component%20Object%20Reference) (Other :type Actor%20Object%20Reference) (OtherComp :type Primitive%20Component%20Object%20Reference) (bSelfMoved :type Boolean) (HitLocation :type Vector :default "0, 0, 0") (HitNormal :type Vector :default "0, 0, 0") (NormalImpulse :type Vector :default "0, 0, 0") (Hit :type Hit%20Result%20Structure%20%28by%20ref%29))
  (Variables|Hit|SetHit Hit)
  (Variables|Hit|SetHitLocation HitLocation)
  (Variables|Hit|SetHitNormal HitNormal)
  (Utilities|FlowControl|Sequence
    (:then_0
      (Hit|ApplyDamagebyProjectile Other OtherComp))
    (:then_3
      (Hit|OnHitEnd))))

(fn ConstructionScript
  (Config|ConfigureProjectileStatsComponent)
  (Config|SetProjectileParameters))

(fn ConfigureProjectileStatsComponent
  (if (!= (Variables|Config|GetProjectileName) "")
    (Utilities|FlowControl|Sequence
      (:then_0
        (Variables|/Game/Gameplay/Components/BPC_Projectile_Stats.BPC_Projectile_Stats_C|SetThisProjectilename (Variables|Default|GetBPC_Projectile_Stats) (Variables|Config|GetProjectileName)))
      (:then_1
        (Default|ConfigureStats (Variables|Default|GetBPC_Projectile_Stats))))))

(fn SetProjectileParameters
  (bind _projectilemovement (Variables|Default|GetProjectileMovement))
  (bind _bpc_projectile_stats (Variables|Default|GetBPC_Projectile_Stats))
  (bind _projectilestats (Variables|/Game/Gameplay/Components/BPC_Projectile_Stats.BPC_Projectile_Stats_C|GetProjectileStats _bpc_projectile_stats))
  (Utilities|FlowControl|Sequence
    (:then_0
      (Variables|/Script/Engine.ProjectileMovementComponent|SetInitialSpeed _projectilemovement (.initialspeed _projectilestats)))
    (:then_1
      (Variables|/Script/Engine.ProjectileMovementComponent|SetMaxSpeed _projectilemovement (.maxspeed _projectilestats)))
    (:then_2
      (Variables|/Script/Engine.ProjectileMovementComponent|SetProjectileGravityScale _projectilemovement (.gravityscale _projectilestats)))))

(fn ApplyDamagebyProjectile
  (params (InActorToDealDamage :type Actor%20Object%20Reference) (In_ATDD_Component :type Primitive%20Component%20Object%20Reference))
  (bind _bpc_projectile_stats (Variables|Default|GetBPC_Projectile_Stats))
  (bind _projectilestats (Variables|/Game/Gameplay/Components/BPC_Projectile_Stats.BPC_Projectile_Stats_C|GetProjectileStats _bpc_projectile_stats))
  (Utilities|FlowControl|Sequence
    (:then_0
      (Utilities|FlowControl|Sequence
        (:then_0
          (LocalVariables|SetL_ProjectileDamageType (.damagetype _projectilestats)))
        (:then_1
          (LocalVariables|SetL_ProjectileDamage (.damage _projectilestats)))))
    (:then_1
      (Game|Damage|ApplyDamage InActorToDealDamage (Math|Conversions|ToFloat(Integer) (LocalVariables|GetL_ProjectileDamage)) 0 (Variables|/Game/Gameplay/Components/BPC_Projectile_Stats.BPC_Projectile_Stats_C|GetOwningWeapon (Variables|Default|GetBPC_Projectile_Stats)) "/Game/Data/Objects/BP_Damage_Base.BP_Damage_Base_C"))))

(fn OnHitEnd
  (Actor|DestroyActor))