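; Base weapon actor that turns Attack and Reload input into charge, shot, reload and cooldown actions.
; SelectAction drives an enum state machine, first checking magazine and spare-mag counts in the owning character's backpack.
; One timeline, rate-scaled by ChargeDuration for every action and reversed for reload and cooldown, triggers the next transition on finish.
; Shots spawn bullet, pellet or rocket projectiles from BPCWeaponStats (work in progress), repeating for automatic fire while input is held.
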(event Custom|ShotAction
  (params (InDuration :type Float%20%28double-precision%29))
  (bind _weaponcurrentstate (Variables|WeaponState|GetWeaponCurrentState))
  ;[0.1719 0.1094 0] ActionProgressTimeline
  (Components|Timeline|SetPlayRate (Variables|Default|GetActionProgressTimeline) (/ 1.0 InDuration))
  (bind _actionprogress (Timeline|ActionProgressTimeline PlayFromStart)
    (:Update
      (Variables|WeaponState|SetActionProgress _actionprogress)
      (switch Utilities|FlowControl|Switch|SwitchonE_Weapon_State _weaponcurrentstate
        (:NewEnumerator1
          (Development|PrintString (Utilities|String|EnumtoString _weaponcurrentstate) :!label _label)
          (Development|PrintString (Utilities|String|ToString(Float) (Variables|WeaponState|GetActionProgress))))
        (:NewEnumerator9
          (CallFunction|ActionProgressTimelineFinishedFunc))
        (:NewEnumerator3
          (goto _label))
        (:NewEnumerator5
          (goto _label))
        (:NewEnumerator6
          (goto _label))))
    (:Finished
      (Development|PrintString (Utilities|String|ToString(Float) (Variables|WeaponState|GetActionProgress)))
      (Variables|WeaponState|SetActionProgress 0.0)
      (switch Utilities|FlowControl|Switch|SwitchonE_Weapon_State (Variables|WeaponState|GetWeaponCurrentState)
        (:NewEnumerator1
          (WeaponState|EndChargeAction))
        (:NewEnumerator3
          (WeaponState|EndShotAction))
        (:NewEnumerator5
          (WeaponState|EndReloadAction))
        (:NewEnumerator6
          (WeaponState|EndCooldownAction))))))

(event Custom|ReloadAction
  (params (InDuration :type Float%20%28double-precision%29))
  (bind _weaponcurrentstate (Variables|WeaponState|GetWeaponCurrentState))
  ;[0.1719 0.1094 0] ActionProgressTimeline
  (Components|Timeline|SetPlayRate (Variables|Default|GetActionProgressTimeline) (/ 1.0 InDuration))
  (bind _actionprogress (Timeline|ActionProgressTimeline ReverseFromEnd)
    (:Update
      (Variables|WeaponState|SetActionProgress _actionprogress)
      (switch Utilities|FlowControl|Switch|SwitchonE_Weapon_State _weaponcurrentstate
        (:NewEnumerator1
          (Development|PrintString (Utilities|String|EnumtoString _weaponcurrentstate) :!label _label)
          (Development|PrintString (Utilities|String|ToString(Float) (Variables|WeaponState|GetActionProgress))))
        (:NewEnumerator9
          (CallFunction|ActionProgressTimelineFinishedFunc))
        (:NewEnumerator3
          (goto _label))
        (:NewEnumerator5
          (goto _label))
        (:NewEnumerator6
          (goto _label))))
    (:Finished
      (Development|PrintString (Utilities|String|ToString(Float) (Variables|WeaponState|GetActionProgress)))
      (Variables|WeaponState|SetActionProgress 0.0)
      (switch Utilities|FlowControl|Switch|SwitchonE_Weapon_State (Variables|WeaponState|GetWeaponCurrentState)
        (:NewEnumerator1
          (WeaponState|EndChargeAction))
        (:NewEnumerator3
          (WeaponState|EndShotAction))
        (:NewEnumerator5
          (WeaponState|EndReloadAction))
        (:NewEnumerator6
          (WeaponState|EndCooldownAction))))))

(event Custom|ChargeAction
  (params (InDuration :type Float%20%28double-precision%29))
  (bind _weaponcurrentstate (Variables|WeaponState|GetWeaponCurrentState))
  ;[0.1719 0.1094 0] ActionProgressTimeline
  (Components|Timeline|SetPlayRate (Variables|Default|GetActionProgressTimeline) (/ 1.0 InDuration))
  (bind _actionprogress (Timeline|ActionProgressTimeline PlayFromStart)
    (:Update
      (Variables|WeaponState|SetActionProgress _actionprogress)
      (switch Utilities|FlowControl|Switch|SwitchonE_Weapon_State _weaponcurrentstate
        (:NewEnumerator1
          (Development|PrintString (Utilities|String|EnumtoString _weaponcurrentstate) :!label _label)
          (Development|PrintString (Utilities|String|ToString(Float) (Variables|WeaponState|GetActionProgress))))
        (:NewEnumerator9
          (CallFunction|ActionProgressTimelineFinishedFunc))
        (:NewEnumerator3
          (goto _label))
        (:NewEnumerator5
          (goto _label))
        (:NewEnumerator6
          (goto _label))))
    (:Finished
      (Development|PrintString (Utilities|String|ToString(Float) (Variables|WeaponState|GetActionProgress)))
      (Variables|WeaponState|SetActionProgress 0.0)
      (switch Utilities|FlowControl|Switch|SwitchonE_Weapon_State (Variables|WeaponState|GetWeaponCurrentState)
        (:NewEnumerator1
          (WeaponState|EndChargeAction))
        (:NewEnumerator3
          (WeaponState|EndShotAction))
        (:NewEnumerator5
          (WeaponState|EndReloadAction))
        (:NewEnumerator6
          (WeaponState|EndCooldownAction))))))

(event Custom|CooldownAction
  (params (InDuration :type Float%20%28double-precision%29))
  (bind _weaponcurrentstate (Variables|WeaponState|GetWeaponCurrentState))
  ;[0.1719 0.1094 0] ActionProgressTimeline
  (Components|Timeline|SetPlayRate (Variables|Default|GetActionProgressTimeline) (/ 1.0 InDuration))
  (bind _actionprogress (Timeline|ActionProgressTimeline ReverseFromEnd)
    (:Update
      (Variables|WeaponState|SetActionProgress _actionprogress)
      (switch Utilities|FlowControl|Switch|SwitchonE_Weapon_State _weaponcurrentstate
        (:NewEnumerator1
          (Development|PrintString (Utilities|String|EnumtoString _weaponcurrentstate) :!label _label)
          (Development|PrintString (Utilities|String|ToString(Float) (Variables|WeaponState|GetActionProgress))))
        (:NewEnumerator9
          (CallFunction|ActionProgressTimelineFinishedFunc))
        (:NewEnumerator3
          (goto _label))
        (:NewEnumerator5
          (goto _label))
        (:NewEnumerator6
          (goto _label))))
    (:Finished
      (Development|PrintString (Utilities|String|ToString(Float) (Variables|WeaponState|GetActionProgress)))
      (Variables|WeaponState|SetActionProgress 0.0)
      (switch Utilities|FlowControl|Switch|SwitchonE_Weapon_State (Variables|WeaponState|GetWeaponCurrentState)
        (:NewEnumerator1
          (WeaponState|EndChargeAction))
        (:NewEnumerator3
          (WeaponState|EndShotAction))
        (:NewEnumerator5
          (WeaponState|EndReloadAction))
        (:NewEnumerator6
          (WeaponState|EndCooldownAction))))))

(event EventBeginPlay)

(event Collision|EventActorBeginOverlap
  (params (OtherActor :type Actor%20Object%20Reference)))

(event EventInteractwithWeapon
  (params (InProcess :type Boolean) (InAction :type E_Character_ActionType%20Enum :default "NewEnumerator3"))
  ;[0.02604 0.000949 0.000949] BPI_Actions: InteractWithWeapon
  (Variables|Input|SetInputActionType InAction)
  (Variables|Input|SetInputInProcess InProcess)
  (if (Variables|Input|GetInputInProcess)
    (switch Utilities|FlowControl|Switch|SwitchonE_Character_ActionType (Variables|Input|GetInputActionType)
      (:NewEnumerator1
        (Variables|WeaponState|SetWeaponCurrentState "NewEnumerator0")
        (WeaponState|SelectAction))
      (:NewEnumerator7
        (Variables|WeaponState|SetWeaponCurrentState "NewEnumerator5")
        (WeaponState|SelectAction)))
    (elif (Utilities|Enum|Equal(Enum) (Variables|WeaponState|GetWeaponCurrentState) "NewEnumerator1")
      (Variables|WeaponState|SetWeaponCurrentState "NewEnumerator9")
      (WeaponState|SelectAction))))

(event EventTick
  (params (DeltaSeconds :type Float%20%28single-precision%29)))

(fn ConstructionScript)

(fn UpdateWeaponAmmo
  (bind _bpc_weapon_stats (Variables|Default|GetBPC_Weapon_Stats))
  (if (Variables|/Game/Gameplay/Components/BPC_Weapon_Stats.BPC_Weapon_Stats_C|GetIsConfigured (Variables|Default|GetBPC_Weapon_Stats))
    (bind _asbp_weapon_base (Utilities|Casting|CastToBP_Weapon_Base (Components|GetOwner))
      (:then
        (bind _asbp_character_base (Utilities|Casting|CastToBP_Character_Base (Components|GetOwner _asbp_weapon_base))
          (:then
            (bind _bpc_character_backpack (Variables|/Game/Gameplay/Characters/BP_Character_Base.BP_Character_Base_C|GetBPC_Character_Backpack _asbp_character_base)
              (:then
                (if (.ReturnValue (Utilities|Map|Find (Variables|/Game/Gameplay/Components/BPC_Character_Backpack.BPC_Character_Backpack_C|GetWeaponry _bpc_character_backpack) (Variables|/Game/Gameplay/Components/BPC_Weapon_Stats.BPC_Weapon_Stats_C|GetWeaponName _bpc_weapon_stats)))
                  (Variables|WeaponState|SetWeapon_CurrentMagFill (.Value (Utilities|Map|Find (Variables|/Game/Gameplay/Components/BPC_Character_Backpack.BPC_Character_Backpack_C|GetWeaponry _bpc_character_backpack) (Variables|/Game/Gameplay/Components/BPC_Weapon_Stats.BPC_Weapon_Stats_C|GetWeaponName _bpc_weapon_stats))))
                  (if (.ReturnValue (Utilities|Map|Find (Variables|/Game/Gameplay/Components/BPC_Character_Backpack.BPC_Character_Backpack_C|GetConsumables _bpc_character_backpack) (Utilities|Struct|BreakF_Weapon_MainStats (Variables|/Game/Gameplay/Components/BPC_Weapon_Stats.BPC_Weapon_Stats_C|GetWeaponMainStats _bpc_weapon_stats))))
                    (Variables|WeaponState|SetWeapon_MagsInBackpack (.Value (Utilities|Map|Find (Variables|/Game/Gameplay/Components/BPC_Character_Backpack.BPC_Character_Backpack_C|GetConsumables _bpc_character_backpack) (Utilities|Struct|BreakF_Weapon_MainStats (Variables|/Game/Gameplay/Components/BPC_Weapon_Stats.BPC_Weapon_Stats_C|GetWeaponMainStats _bpc_weapon_stats)))))
                    (return true)
                    (else
                      _))))
              (:else
                _)))
          (:CastFailed
            _)))
      (:CastFailed
        _)))
  (return false))

(fn UpdateWeaponAvailability
  (bind _success (Update|UpdateWeaponAmmo))
  (if _success
    (if (> (Variables|WeaponState|GetWeapon_CurrentMagFill) 0)
      _
      (elif (> (Variables|WeaponState|GetWeapon_MagsInBackpack) 0)
        (Variables|WeaponState|SetWeaponCurrentState "NewEnumerator4")
        (else
          (Variables|WeaponState|SetWeaponCurrentState "NewEnumerator7")
          (return false))))
    (return true)
    (else
      (Variables|WeaponState|SetWeaponCurrentState "NewEnumerator7")
      (return false))))

(fn SelectAction
  (Update|UpdateWeaponAvailability)
  (if (Utilities|Enum|NotEqual(Enum) (Variables|WeaponState|GetWeaponCurrentState) "NewEnumerator7")
    (Utilities|FlowControl|Sequence
      (:then_0
        (switch Utilities|FlowControl|Switch|SwitchonE_Weapon_State (Variables|WeaponState|GetWeaponCurrentState)
          (:NewEnumerator0
            (WeaponState|StartChargeAction))
          (:NewEnumerator9
            (WeaponState|CancelChargeAction))
          (:NewEnumerator2
            (WeaponState|StartShotAction))
          (:NewEnumerator4
            (WeaponState|CheckWeaponReloadActionType))
          (:NewEnumerator5
            (WeaponState|StartReloadAction))
          (:NewEnumerator6
            (WeaponState|StartCooldownAction)))))
    (else
      (Development|PrintString "Weapon Is NOT READY!!!"))))

(fn StartChargeAction
  (Variables|WeaponState|SetWeaponCurrentState "NewEnumerator1")
  (CallFunction|ChargeAction (Utilities|Struct|BreakF_Weapon_MainStats (Variables|/Game/Gameplay/Components/BPC_Weapon_Stats.BPC_Weapon_Stats_C|GetWeaponMainStats (Variables|Default|GetBPC_Weapon_Stats)))))

(fn EndChargeAction
  (Variables|WeaponState|SetWeaponCurrentState "NewEnumerator2")
  (WeaponState|SelectAction))

(fn CancelChargeAction
  (Variables|WeaponState|SetWeaponCurrentState "NewEnumerator6")
  (WeaponState|SelectAction))

(fn StartShotAction
  (Variables|WeaponState|SetWeaponCurrentState "NewEnumerator3")
  (Projectile|SpawnProjectile)
  (CallFunction|ShotAction (Utilities|Struct|BreakF_Weapon_MainStats (Variables|/Game/Gameplay/Components/BPC_Weapon_Stats.BPC_Weapon_Stats_C|GetWeaponMainStats (Variables|Default|GetBPC_Weapon_Stats)))))

(fn SpawnProjectile
  (bind _bpc_weapon_stats (Variables|Default|GetBPC_Weapon_Stats))
  (bind _bpc_weapon_stats_2 (Variables|Default|GetBPC_Weapon_Stats))
  (bind _bpc_weapon_stats_3 (Variables|Default|GetBPC_Weapon_Stats))
  (bind _weaponprojectilestats (Variables|/Game/Gameplay/Components/BPC_Weapon_Stats.BPC_Weapon_Stats_C|GetWeaponProjectileStats _bpc_weapon_stats))
  (bind _weaponprojectilestats_2 (Variables|/Game/Gameplay/Components/BPC_Weapon_Stats.BPC_Weapon_Stats_C|GetWeaponProjectileStats _bpc_weapon_stats_2))
  (bind _weaponprojectilestats_3 (Variables|/Game/Gameplay/Components/BPC_Weapon_Stats.BPC_Weapon_Stats_C|GetWeaponProjectileStats _bpc_weapon_stats_3))
  (bind (_effecttype _damage _damagetype _initialspeed _maxspeed _gravityscale _homingmagnitude) (Utilities|Struct|BreakF_Projectile_MainStats _weaponprojectilestats_2))
  (bind (_effecttype_2 _damage_2 _damagetype_2 _initialspeed_2 _maxspeed_2 _gravityscale_2 _homingmagnitude_2) (Utilities|Struct|BreakF_Projectile_MainStats _weaponprojectilestats_3))
  (bind (_effecttype_3 _damage_3 _damagetype_3 _initialspeed_3 _maxspeed_3 _gravityscale_3 _homingmagnitude_3) (Utilities|Struct|BreakF_Projectile_MainStats _weaponprojectilestats))
  ;[1 0.02083 0.02083] InProgress
  (switch Utilities|FlowControl|Switch|SwitchonE_Projectile_Type (Utilities|Struct|BreakF_Projectile_MainStats (Variables|/Game/Gameplay/Components/BPC_Weapon_Stats.BPC_Weapon_Stats_C|GetWeaponProjectileStats (Variables|Default|GetBPC_Weapon_Stats)))
    (:NewEnumerator0
      ;;[1 1 1] Bullet
      (Game|SpawnActorfromClass "/Game/Gameplay/Weapons/Projectiles/BP_Projectile_Bullet.BP_Projectile_Bullet_C" (Transformation|GetWorldTransform (Variables|Default|GetWeaponMuzzle)) "Undefined" "OverrideRootScale" self _effecttype_2 _damage_2 _damagetype_2 _initialspeed_2 _maxspeed_2 _gravityscale_2 _homingmagnitude_2 0))
    (:NewEnumerator1
      ;;[1 1 1] Pellets
      (Game|SpawnActorfromClass "/Game/Gameplay/Weapons/Projectiles/BP_Projectile_Pellet.BP_Projectile_Pellet_C" (Transformation|GetWorldTransform (Variables|Default|GetWeaponMuzzle)) "Undefined" "OverrideRootScale" self _effecttype_3 _damage_3 _damagetype_3 _initialspeed_3 _maxspeed_3 _gravityscale_3 _homingmagnitude_3 0))
    (:NewEnumerator2
      ;;[1 1 1] Rocket
      (Game|SpawnActorfromClass "/Game/Gameplay/Weapons/Projectiles/BP_Projectile_Rocket.BP_Projectile_Rocket_C" (Transformation|GetWorldTransform (Variables|Default|GetWeaponMuzzle)) "Undefined" "OverrideRootScale" self _effecttype _damage _damagetype _initialspeed _maxspeed _gravityscale _homingmagnitude 0))))

(fn EndShotAction
  (if (Variables|Input|GetInputInProcess)
    (switch Utilities|FlowControl|Switch|SwitchonE_Weapon_ShotType (Utilities|Struct|BreakF_Weapon_MainStats (Variables|/Game/Gameplay/Components/BPC_Weapon_Stats.BPC_Weapon_Stats_C|GetWeaponMainStats (Variables|Default|GetBPC_Weapon_Stats)))
      (:NewEnumerator8
        (Variables|WeaponState|SetWeaponCurrentState "NewEnumerator6" :!label _label)
        (WeaponState|SelectAction))
      (:NewEnumerator9
        (Variables|WeaponState|SetWeaponCurrentState "NewEnumerator2")
        (WeaponState|SelectAction))
      (:NewEnumerator10
        (goto _label))
      (:NewEnumerator11
        (goto _label)))
    (else
      (goto _label))))

(fn StartReloadAction
  (Variables|WeaponState|SetWeaponCurrentState "NewEnumerator5")
  (CallFunction|ReloadAction (Utilities|Struct|BreakF_Weapon_MainStats (Variables|/Game/Gameplay/Components/BPC_Weapon_Stats.BPC_Weapon_Stats_C|GetWeaponMainStats (Variables|Default|GetBPC_Weapon_Stats)))))

(fn EndReloadAction
  (Variables|WeaponState|SetWeaponCurrentState "NewEnumerator0")
  (WeaponState|SelectAction))

(fn CheckWeaponReloadActionType
  (switch Utilities|FlowControl|Switch|SwitchonE_Weapon_ReloadType (.ReloadType (Utilities|Struct|BreakF_Weapon_MainStats (Variables|/Game/Gameplay/Components/BPC_Weapon_Stats.BPC_Weapon_Stats_C|GetWeaponMainStats (Variables|Default|GetBPC_Weapon_Stats))))
    (:NewEnumerator2
      (Variables|WeaponState|SetWeaponCurrentState "NewEnumerator5")
      (WeaponState|SelectAction))))

(fn StartCooldownAction
  (Variables|WeaponState|SetWeaponCurrentState "NewEnumerator6")
  (CallFunction|CooldownAction (Utilities|Struct|BreakF_Weapon_MainStats (Variables|/Game/Gameplay/Components/BPC_Weapon_Stats.BPC_Weapon_Stats_C|GetWeaponMainStats (Variables|Default|GetBPC_Weapon_Stats)))))

(fn EndCooldownAction
  (Variables|WeaponState|SetWeaponCurrentState "NewEnumerator0")
  (WeaponState|SelectAction))

(fn InteractwithObjects
  (params (InitiatedActor :type Actor%20Object%20Reference))
  (return false))