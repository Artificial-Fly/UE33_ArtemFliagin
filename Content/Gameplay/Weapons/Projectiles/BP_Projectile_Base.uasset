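; Base projectile actor for weapons that damages characters on hit and then destroys itself.
; The construction script copies its speed and gravity settings into the ProjectileMovement component.
; On hit it prints a debug message, damages BP_Character_Base targets with a class chosen by element (only Arcane differs from base), runs an effect switch, then destroys itself.
; The effect switch is a stub with only a No Effect case shown.
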(event EventBeginPlay)

(event Collision|EventActorBeginOverlap
  (params (OtherActor :type Actor%20Object%20Reference)))

(event EventTick
  (params (DeltaSeconds :type Float%20%28single-precision%29)))

(event Collision|EventHit
  (params (MyComp :type Primitive%20Component%20Object%20Reference) (Other :type Actor%20Object%20Reference) (OtherComp :type Primitive%20Component%20Object%20Reference) (bSelfMoved :type Boolean) (HitLocation :type Vector :default "0, 0, 0") (HitNormal :type Vector :default "0, 0, 0") (NormalImpulse :type Vector :default "0, 0, 0") (Hit :type Hit%20Result%20Structure%20%28by%20ref%29))
  (Variables|Default|SetOther Other)
  (Variables|Default|SetHitLocation HitLocation)
  (Variables|Default|SetHitNormal HitNormal)
  (Variables|Default|SetHit Hit)
  (Development|PrintString "HIT!" true true "(R=1.000000,G=0.165070,B=0.000000,A=1.000000)")
  (Utilities|FlowControl|Sequence
    (:then_0
      (CallFunction|DealDamagebyProjectile))
    (:then_1
      (CallFunction|ProjectileEffect))
    (:then_2
      (CallFunction|DestroyThisProjectile))))

(fn ConstructionScript
  (bind _projectilemovement (Variables|Default|GetProjectileMovement))
  (Variables|/Script/Engine.ProjectileMovementComponent|SetInitialSpeed _projectilemovement (Variables|Default|GetInitialSpeed))
  (Variables|/Script/Engine.ProjectileMovementComponent|SetMaxSpeed _projectilemovement (Variables|Default|GetMaxSpeed))
  (Variables|/Script/Engine.ProjectileMovementComponent|SetProjectileGravityScale _projectilemovement (Variables|Default|GetGravityScale)))

(fn DealDamagebyProjectile
  (Utilities|Casting|CastToBP_Character_Base (Variables|Default|GetOther))
  (Utilities|FlowControl|Sequence
    (:then_0)
    (:then_1
      (Game|Damage|ApplyDamage (Variables|Default|GetOther) (Math|Conversions|ToFloat(Integer) (Variables|Default|GetDamage)) 0 self (Utilities|Select :Index (Variables|Default|GetProjectileDamageType) :NewEnumerator0 "/Game/Data/Objects/BP_Damage_Arcane.BP_Damage_Arcane_C" :NewEnumerator1 "/Game/Data/Objects/BP_Damage_Base.BP_Damage_Base_C" :NewEnumerator2 "/Game/Data/Objects/BP_Damage_Base.BP_Damage_Base_C" :NewEnumerator3 "/Game/Data/Objects/BP_Damage_Base.BP_Damage_Base_C" :NewEnumerator4 "/Game/Data/Objects/BP_Damage_Base.BP_Damage_Base_C")))))

(fn ProjectileEffect
  (switch Utilities|FlowControl|Switch|SwitchonE_Projectile_EffectType (Variables|Default|GetProjectileEffectType)
    (:NewEnumerator0
      (return))))

(fn DestroyThisProjectile
  (Actor|DestroyActor))