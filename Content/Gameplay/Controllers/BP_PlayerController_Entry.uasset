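; Player controller that sets the game's pause and mouse-input state based on whether the in-game UI is showing.
; BeginPlay caches the controlled pawn and the BP_HUD_Base reference, then updates that state after a short delay.
; Without a top-level WBP_InGameUI widget, the game pauses and enables the cursor, click and mouse-over events.
; A self-damage call on the pawn is left unconnected.
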(event EventBeginPlay
  ;[0.02122 0.02122 0.02122] Getting player's pawn/character (BP_Character_Player in this case)
  (Variables|PlayerControllerConfig|SetControlledPawn (Pawn|GetControlledPawn))
  ;;[0 0 0] PLACE HUD UPDATE HERE
  (Update|UpdateCurrentHUD)
  (Utilities|FlowControl|Delay 3.0)
  (Update|UpdateGamePauseState))

(event EventTick
  (params (DeltaSeconds :type Float%20%28single-precision%29)))

(event Input|KeyboardEvents|DebugKey2
  (params (Key :type Key%20Structure) (ActionValue :type Input%20Action%20Value%20Structure))
  ;[0 0 0] Comment
)

(fn ConstructionScript)

(fn UpdateGamePauseState
  (bind _output_get (LocalVariables|SetIsCurrentWidgetNotInGame (not (CallFunction|GetIsCurrentWidgetinGame))))
  (Game|SetGamePaused _output_get)
  (Variables|Default|SetbShowMouseCursor (LocalVariables|GetIsCurrentWidgetNotInGame))
  (Variables|Default|SetbEnableClickEvents (LocalVariables|GetIsCurrentWidgetNotInGame))
  (Variables|Default|SetbEnableMouseOverEvents (LocalVariables|GetIsCurrentWidgetNotInGame)))

(fn UpdateCurrentHUD
  (Utilities|FlowControl|Sequence
    (:then_0
      (Variables|HUD|GetCurrentHUD
        (:then)
        (:else
          (bind _asbp_hud_base (Utilities|Casting|CastToBP_HUD_Base (HUD|GetHUD)))
          (Variables|HUD|SetCurrentHUD _asbp_hud_base))))
    (:then_1
      (return))))

(fn GetIsCurrentWidgetinGame
  (bind _foundwidgets (Widget|GetAllWidgetsOfClass "/Game/Gameplay/HUD/Widgets/SessionScreen/WBP_InGameUI.WBP_InGameUI_C" true))
  (return (Utilities|Array|IsNotEmpty _foundwidgets)))