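; Weapon stats component that loads a weapon's configuration from data tables when play begins.
; ConfigureWeaponStats looks up the main stats row by WeaponName, then uses row names stored in it to fetch the magazine and projectile stat rows.
; Each row is cached on the component, and IsConfigured turns true only if all three lookups succeed; an unset name or missing row sets it false.
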(event EventBeginPlay
  (CallFunction|ConfigureWeaponStats))

(event EventTick
  (params (DeltaSeconds :type Float%20%28single-precision%29)))

(fn ConfigureWeaponStats
  (if (!= (Variables|Config|GetWeaponName) "")
    (bind _returnvalue (Utilities|GetDataTableRow "/Game/Data/DataTables/DT_Weapons_MainStats.DT_Weapons_MainStats" (Variables|Config|GetWeaponName))
      (:then
        (bind _output_get (Variables|WeaponDTStats|SetWeaponMainStats _returnvalue))
        (bind _returnvalue_2 (Utilities|GetDataTableRow "/Game/Data/DataTables/DT_Weapons_MagStats.DT_Weapons_MagStats" (.MagDTName (Utilities|Struct|BreakF_Weapon_MainStats _output_get)))
          (:then
            (Variables|WeaponDTStats|SetWeaponMagStats _returnvalue_2)
            (bind _returnvalue_3 (Utilities|GetDataTableRow "/Game/Data/DataTables/DT_Projectile_Mainstats.DT_Projectile_Mainstats" (.ProjectileDTName (Utilities|Struct|BreakF_Weapon_MainStats _output_get)))
              (:then
                (Variables|WeaponDTStats|SetWeaponProjectileStats _returnvalue_3)
                (Variables|Config|SetIsConfigured true))
              (:RowNotFound
                (Variables|Config|SetIsConfigured false :!label _label))))
          (:RowNotFound
            (goto _label))))
      (:RowNotFound
        (goto _label)))
    (else
      (goto _label))))