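; Character component that holds main stats and health, loaded on BeginPlay from DT_Characters_MainStats by CurrentCharacter name, rejecting NonNPC types.
; It stores gait coefficients and sets the owning BP_Character_Base's walk and crouch speeds.
; HP starts at maximum, except that a player in a continued game restores saved HP from the game instance.
; RecieveDamage and HealUP update HP and broadcast stat changes, with damage also setting the death flag.
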(event EventBeginPlay
  (Config|ConfigureStats))

(event EventTick
  (params (DeltaSeconds :type Float%20%28single-precision%29)))

(fn ConfigureStats
  (if (!= (Variables|Config|GetCurrentCharacter) "")
    (bind _returnvalue (Utilities|GetDataTableRow "/Game/Data/DataTables/DT_Characters_MainStats.DT_Characters_MainStats" (Variables|Config|GetCurrentCharacter))
      (:then
        (Variables|Config|SetCharacterStats _returnvalue)
        (if (Utilities|Enum|NotEqual(Enum) (.Type (Utilities|Struct|BreakF_Character_MainStats (Variables|Config|GetCharacterStats))) "NewEnumerator4")
          (Utilities|FlowControl|Sequence
            (:then_0
              (Config|ConfigureMovementStats))
            (:then_1
              (Config|ConfigureHP)))
          (else
            (Development|PrintString "ConfigureStats error: This character has NonNPC type!"))))
      (:RowNotFound
        (Development|PrintString "ConfigureStats error: CurrentCharacter hasn't been found in DT_Characters_Stats")))
    (else
      (Development|PrintString "ConfigureStats error: CurrentCharacter is invalid"))))

(fn ConfigureMovementStats
  (bind _characterstats (Variables|Config|GetCharacterStats))
  (bind _characterstats_2 (Variables|Config|GetCharacterStats))
  (bind _maxwalkspeed (Utilities|Struct|BreakF_Character_MainStats _characterstats))
  (bind (_walkkoef _runkoef _aimkoef _crouchkoef) (Utilities|Struct|BreakF_Character_MainStats _characterstats_2))
  (bind _asbp_character_base (Utilities|Casting|CastToBP_Character_Base (Components|GetOwner)))
  (LocalVariables|SetL_Character _asbp_character_base)
  (Utilities|FlowControl|Sequence
    (:then_0
      ;[0.02083 0.02083 0.02083] Set Movement Coefficients
      (Utilities|FlowControl|Sequence
        (:then_0
          (Variables|Config|SetCharacterWalkKoeff _walkkoef))
        (:then_1
          (Variables|Config|SetCharacterRunKoeff _runkoef))
        (:then_2
          (Variables|Config|SetCharacterAimKoeff _aimkoef))
        (:then_3
          (Variables|Config|SetCharacterCrouchKoeff _crouchkoef))))
    (:then_1
      ;[0.03646 0.03646 0.03646] Set Movement Component Parameters
      (Variables|/Script/Engine.CharacterMovementComponent|SetMaxWalkSpeed (Variables|/Script/Engine.Character|GetCharacterMovement (LocalVariables|GetL_Character)) _maxwalkspeed)
      (Variables|/Script/Engine.CharacterMovementComponent|SetMaxWalkSpeedCrouched (Variables|/Script/Engine.Character|GetCharacterMovement (LocalVariables|GetL_Character)) (* _maxwalkspeed (Variables|Config|GetCharacterCrouchKoeff))))))

(fn ConfigureHP
  (bind _asbp_game_instance (Utilities|Casting|CastToBP_GameInstance (Game|GetGameInstance)))
  (if (not (Variables|/Game/Gameplay/BP_GameInstance.BP_GameInstance_C|GetIsItNewGame _asbp_game_instance))
    (bind _game_savedata (Utilities|CheckSaveSlot)
      (:IsValid
        (Variables|Update|SetCurrentHP (Math|Integer|Min(Integer) (.maxhp (Variables|Config|GetCharacterStats)) (Variables|/Game/Data/Objects/BP_Game_SaveData.BP_Game_SaveData_C|GetSavedPlayer_CurrentHP _game_savedata)))
        (Default|CallOnStatsUpdated (.maxhp (Variables|Config|GetCharacterStats)) (Variables|Update|GetCurrentHP) (Variables|Update|GetisDead) false))
      (:IsNotValid
        (Update|HealUP true :!label _label)))
    (else
      (goto _label))))

(fn RecieveDamage
  (params (InDamage :type Integer) (InType :type E_Element_Type%20Enum :default "NewEnumerator0") (InCauser :type Actor%20Object%20Reference))
  (if (not (Variables|Update|GetisDead))
    (Variables|Update|SetCurrentHP (- (Variables|Update|GetCurrentHP) InDamage))
    (Variables|Update|SetisDead (not (> (Variables|Update|GetCurrentHP) 0)))
    (Default|CallOnStatsUpdated (.MaxHP (Utilities|Struct|BreakF_Character_MainStats (Variables|Config|GetCharacterStats))) (Variables|Update|GetCurrentHP) (Variables|Update|GetisDead) true)))

(fn HealUP
  (params (InIsToMaxHP :type Boolean) (InAddHP :type Integer))
  (if InIsToMaxHP
    (Variables|Update|SetCurrentHP (.MaxHP (Utilities|Struct|BreakF_Character_MainStats (Variables|Config|GetCharacterStats))))
    (else
      (Variables|Update|SetCurrentHP (Math|Integer|Min(Integer) (+ (Variables|Update|GetCurrentHP) InAddHP) (.MaxHP (Utilities|Struct|BreakF_Character_MainStats (Variables|Config|GetCharacterStats)))))))
  (Default|CallOnStatsUpdated (.MaxHP (Utilities|Struct|BreakF_Character_MainStats (Variables|Config|GetCharacterStats))) (Variables|Update|GetCurrentHP) (Variables|Update|GetisDead) false))

(fn CheckHP
  (return (>= (Variables|Update|GetCurrentHP) (.MaxHP (Utilities|Struct|BreakF_Character_MainStats (Variables|Config|GetCharacterStats))))))

(fn GetStats
  (bind _characterstats (Variables|Config|GetCharacterStats))
  (bind (_type _maxhp _maxwalkspeed _damagekoef _senseradius) (Utilities|Struct|BreakF_Character_MainStats _characterstats))
  (return (Variables|Config|GetCurrentCharacter) _type (Variables|Update|GetisDead) _maxhp (Variables|Update|GetCurrentHP) _maxwalkspeed _damagekoef _senseradius))