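; Character backpack component that stores keys, quest items, consumables and weapons, broadcasting updates after AddNewItem and shortly after BeginPlay.
; AddNewItem routes by item type, though quest item and consumable handlers are empty stubs.
; AddNewWeapon caches weapon type and magazine limits from data tables into name-keyed maps, then fills the magazine.
; Spare magazines are clamped counts in Consumables; RemoveKey targets QuestItems, and magazine-fill subtraction is never written back.
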(event EventBeginPlay
  (Utilities|FlowControl|Delay 3.0)
  (Default|CallOnBackPackUpdated (Variables|Key|GetKeys) (Variables|Quest|GetQuestItems) (Variables|Consumables|GetConsumables) (Variables|Weapons|GetWeaponry)))

(event EventTick
  (params (DeltaSeconds :type Float%20%28single-precision%29)))

(fn AddNewItem
  (params (InItemName :type Name) (InItemType :type E_Pickup_Type%20Enum :default "NewEnumerator0"))
  (Utilities|FlowControl|Sequence
    (:then_0
      (switch Utilities|FlowControl|Switch|SwitchonE_Pickup_Type InItemType
        (:NewEnumerator4
          (Development|PrintString "Failed to add new item to Inventory: unknown type of item"))
        (:NewEnumerator0
          (key|AddNewKey InItemName))
        (:NewEnumerator1
          (Quest|AddQuestItem))
        (:NewEnumerator2
          (Consumables|AddConsumable))
        (:NewEnumerator3
          (Weapons|AddNewWeapon InItemName))))
    (:then_1
      (Default|CallOnBackPackUpdated (Variables|Key|GetKeys) (Variables|Quest|GetQuestItems) (Variables|Consumables|GetConsumables) (Variables|Weapons|GetWeaponry)))))

(fn AddNewKey
  (params (InNewKey :type Name))
  (Utilities|Set|Add (Variables|Key|GetKeys) InNewKey)
  (return true))

(fn RemoveKey
  (params (InKeyToRemove :type Name))
  (bind _returnvalue (Utilities|Set|Remove (Variables|Quest|GetQuestItems) InKeyToRemove))
  (return _returnvalue))

(fn AddQuestItem)

(fn RemoveQuestItem)

(fn AddConsumable)

(fn RemoveConsumable)

(fn AddNewWeapon
  (params (InWeaponName :type Name :default "TestWeapon"))
  (if (!= InWeaponName "")
    (bind _returnvalue (Utilities|GetDataTableRow "/Game/Data/DataTables/DT_Weapons_MainStats.DT_Weapons_MainStats" InWeaponName)
      (:then
        (bind _output_get (LocalVariables|SetWeapon_DTMainStats _returnvalue))
        (LocalVariables|SetWeapon_WeaponType (.WeaponType (Utilities|Struct|BreakF_Weapon_MainStats _output_get)))
        (bind _returnvalue_2 (Utilities|GetDataTableRow "/Game/Data/DataTables/DT_Weapons_MagStats.DT_Weapons_MagStats" (.MagDTName (Utilities|Struct|BreakF_Weapon_MainStats _output_get)))
          (:then
            (bind _output_get_2 (LocalVariables|SetWeapon_DTMagStats _returnvalue_2))
            ;[1 1 1] Max number for Weaponry Int
            (Utilities|Map|Add (Variables|Weapons|GetMagName_MagCapacity) (.MagDTName (Utilities|Struct|BreakF_Weapon_MainStats _output_get)) (.MagCapacity (Utilities|Struct|BreakF_Weapon_MagStats _output_get_2)))
            ;[1 1 1] Max number of Mag in Backpack
            (Utilities|Map|Add (Variables|Weapons|GetMagName_MagMaxNumber) (.MagDTName (Utilities|Struct|BreakF_Weapon_MainStats _output_get)) (.MagMaxNumber (Utilities|Struct|BreakF_Weapon_MagStats _output_get_2)))
            ;[1 1 1] Weapon Name : Mag Name for finding it later
            (Utilities|Map|Add (Variables|Weapons|GetWeaponName_MagName) InWeaponName (.MagDTName (Utilities|Struct|BreakF_Weapon_MainStats _output_get)))
            ;[1 1 1] Weapon Name : Current Mag Fill
            (Utilities|Map|Add (Variables|Weapons|GetWeaponry) InWeaponName 100)
            ;[1 1 1] Weapon : Weapon Type
            (Utilities|Map|Add (Variables|Weapons|GetWeaponName_WeaponType) InWeaponName (LocalVariables|GetWeapon_WeaponType))
            (bind _success (Weapons|UpdateWeaponCurrentMagFill InWeaponName true 1))
            (if _success
              (Variables|Weapons|SetLastAddedWeapon InWeaponName)
              (return _success)
              (else
                (return false))))))
      (:RowNotFound
        _)))
  (return false))

(fn RemoveWeapon
  (params (InWeaponName :type Name :default "TestWeapon"))
  (Utilities|Map|Remove (Variables|Weapons|GetWeaponry) InWeaponName))

(fn UpdateWeaponCurrentMagFill
  (params (InWeaponName :type Name :default "TestWeapon") (InResetMagToMaxVal :type Boolean) (InSubstract :type Integer))
  (bind _weaponname_magname (Variables|Weapons|GetWeaponName_MagName))
  (bind _magname_magcapacity (Variables|Weapons|GetMagName_MagCapacity))
  (bind _weaponry (Variables|Weapons|GetWeaponry))
  (bind (_value _returnvalue) (Utilities|Map|Find _weaponry InWeaponName))
  (bind (_value_2 _returnvalue_2) (Utilities|Map|Find _weaponname_magname InWeaponName))
  (bind (_value_3 _returnvalue_3) (Utilities|Map|Find _magname_magcapacity _value_2))
  (if (not (Math|Boolean|ANDBoolean _returnvalue _returnvalue_2 _returnvalue_3))
    (return false)
    (else
      (LocalVariables|SetL_CurrentMagFill _value)
      (LocalVariables|SetL_CurrentMagCapacity _value_3)
      (if InResetMagToMaxVal
        (Utilities|Map|Add (Variables|Weapons|GetWeaponry) InWeaponName (LocalVariables|GetL_CurrentMagCapacity))
        (return true)
        (else
          (LocalVariables|SetL_CurrentMagFill (Math|Integer|Min(Integer) (Math|Integer|Max(Integer) (- (LocalVariables|GetL_CurrentMagFill) InSubstract)) (LocalVariables|GetL_CurrentMagCapacity)))
          (return true))))))

(fn UpdateWeaponMagsinBackpack
  (params (InWeaponName :type Name :default "TestWeapon") (InResetToMaxVal :type Boolean) (InSubstract :type Integer))
  (bind _weaponname_magname (Variables|Weapons|GetWeaponName_MagName))
  (bind (_value _returnvalue) (Utilities|Map|Find _weaponname_magname InWeaponName))
  (if _returnvalue
    (LocalVariables|SetL_MagName _value)
    (if (.ReturnValue (Utilities|Map|Find (Variables|Weapons|GetMagName_MagMaxNumber) (LocalVariables|GetL_MagName)))
      (LocalVariables|SetL_MaxMagsInBackpackNumber (.Value (Utilities|Map|Find (Variables|Weapons|GetMagName_MagMaxNumber) (LocalVariables|GetL_MagName))))
      (if (.ReturnValue (Utilities|Map|Find (Variables|Consumables|GetConsumables) (LocalVariables|GetL_MagName)))
        (LocalVariables|SetL_CurrentMagsInBackpackNumber (.Value (Utilities|Map|Find (Variables|Consumables|GetConsumables) (LocalVariables|GetL_MagName))))
        (else
          (LocalVariables|SetL_CurrentMagsInBackpackNumber 0)))
      (if InResetToMaxVal
        (Utilities|Map|Add (Variables|Consumables|GetConsumables) (LocalVariables|GetL_MagName) (LocalVariables|GetL_MaxMagsInBackpackNumber))
        (return true)
        (else
          (LocalVariables|SetL_CurrentMagsInBackpackNumber (Math|Integer|Min(Integer) (Math|Integer|Max(Integer) (- (LocalVariables|GetL_CurrentMagsInBackpackNumber) InSubstract)) (LocalVariables|GetL_MaxMagsInBackpackNumber)))
          (Utilities|Map|Add (Variables|Consumables|GetConsumables) (LocalVariables|GetL_MagName) (LocalVariables|GetL_CurrentMagsInBackpackNumber))
          (return true)))
      (else
        _)))
  (return false))