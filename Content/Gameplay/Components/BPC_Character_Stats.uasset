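; Actor component that holds a character's stats and tracks its health, damage, healing and death.
; On BeginPlay it loads the CurrentCharacter row from DT_Characters_Stats, rejects one excluded type, and sets the owning BP_Character_Base's walk speed, with crouch at half.
; Initial HP setup only clamps CurrentHP to the maximum.
; Damage and healing both broadcast OnStatsUpdated, and GetStats exposes the values to other systems.
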(event EventBeginPlay
  (Config|ConfigureStats))

(event EventTick
  (params (DeltaSeconds :type Float%20%28single-precision%29)))

(fn ConfigureStats
  (if (!= (Variables|Config|GetCurrentCharacter) "")
    (bind _returnvalue (Utilities|GetDataTableRow "/Game/Data/DataTables/DT_Characters_Stats.DT_Characters_Stats" (Variables|Config|GetCurrentCharacter))
      (:then
        (Variables|Config|SetCharacterStats _returnvalue)
        (if (Utilities|Enum|NotEqual(Enum) (Utilities|Struct|BreakSTRUCT_Character_Stats (Variables|Config|GetCharacterStats)) "NewEnumerator4")
          (Utilities|FlowControl|Sequence
            (:then_0
              (Config|ConfigureMovementStats))
            (:then_1
              (Config|ConfigureHP)))
          (else
            (Development|PrintString "ConfigureStats error: This character has NonNPC type!"))))
      (:RowNotFound
        (Development|PrintString "ConfigureStats error: CurrentCharacter hasn't been found in DT_Characters_Stats")))
    (else
      (Development|PrintString "ConfigureStats error: CurrentCharacter is invalid"))))

(fn ConfigureMovementStats
  (bind _characterstats (Variables|Config|GetCharacterStats))
  (bind _maxwalkspeed (Utilities|Struct|BreakSTRUCT_Character_Stats _characterstats))
  (bind _asbp_character_base (Utilities|Casting|CastToBP_Character_Base (Components|GetOwner)))
  (Variables|/Script/Engine.CharacterMovementComponent|SetMaxWalkSpeed (Variables|/Script/Engine.Character|GetCharacterMovement _asbp_character_base) _maxwalkspeed)
  (Variables|/Script/Engine.CharacterMovementComponent|SetMaxWalkSpeedCrouched (Variables|/Script/Engine.Character|GetCharacterMovement _asbp_character_base) (* _maxwalkspeed 0.5)))

(fn ConfigureHP
  (Update|HealUP false))

(fn RecieveDamage
  (params (InDamage :type Integer) (InType :type ENUM_Element_Type%20Enum :default "NewEnumerator0") (InCauser :type Actor%20Object%20Reference))
  (if (not (Variables|Update|GetisDead))
    (Variables|Update|SetCurrentHP (- (Variables|Update|GetCurrentHP) InDamage))
    (Variables|Update|SetisDead (not (> (Variables|Update|GetCurrentHP) 0)))
    (Default|CallOnStatsUpdated (Utilities|Struct|BreakSTRUCT_Character_Stats (Variables|Config|GetCharacterStats)) (Variables|Update|GetCurrentHP) (Variables|Update|GetisDead) true)))

(fn HealUP
  (params (InIsToMaxHP :type Boolean) (InAddHP :type Integer))
  (if InIsToMaxHP
    (Variables|Update|SetCurrentHP (Utilities|Struct|BreakSTRUCT_Character_Stats (Variables|Config|GetCharacterStats)))
    (else
      (Variables|Update|SetCurrentHP (Math|Integer|Min(Integer) (+ (Variables|Update|GetCurrentHP) InAddHP) (Utilities|Struct|BreakSTRUCT_Character_Stats (Variables|Config|GetCharacterStats))))))
  (Default|CallOnStatsUpdated (Utilities|Struct|BreakSTRUCT_Character_Stats (Variables|Config|GetCharacterStats)) (Variables|Update|GetCurrentHP) (Variables|Update|GetisDead) false))

(fn CheckHP
  (return (>= (Variables|Update|GetCurrentHP) (Utilities|Struct|BreakSTRUCT_Character_Stats (Variables|Config|GetCharacterStats)))))

(fn GetStats
  (bind _characterstats (Variables|Config|GetCharacterStats))
  (bind (_type _maxhp _maxwalkspeed _damagekoef _senseradius) (Utilities|Struct|BreakSTRUCT_Character_Stats _characterstats))
  (return (Variables|Config|GetCurrentCharacter) _type (Variables|Update|GetisDead) _maxhp (Variables|Update|GetCurrentHP) _maxwalkspeed _damagekoef _senseradius))