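; Backpack component that serves as an inventory for keys, quest items, consumables and weapons, with only key handling partly implemented.
; AddNewItem switches on item type to call the matching add function, printing an error for unknown types.
; AddNewKey stores names in Keys, but RemoveKey removes from QuestItems instead of Keys.
; The quest item, consumable and weapon functions are empty stubs.
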(event EventBeginPlay)

(event EventTick
  (params (DeltaSeconds :type Float%20%28single-precision%29)))

(fn AddNewItem
  (params (InItemName :type Name) (InItemType :type ENUM_Pickup_Type%20Enum :default "NewEnumerator0"))
  (switch Utilities|FlowControl|Switch|SwitchonENUM_Pickup_Type InItemType
    (:NewEnumerator4
      (Development|PrintString "Failed to add new item to Inventory: unknown type of item"))
    (:NewEnumerator0
      (key|AddNewKey InItemName))
    (:NewEnumerator1
      (Quest|AddQuestItem))
    (:NewEnumerator2
      (Consumables|AddConsumable))
    (:NewEnumerator3
      (Weapons|AddNewWeapon))))

(fn AddNewKey
  (params (InNewKey :type Name))
  (Utilities|Set|Add (Variables|Key|GetKeys) InNewKey)
  (return true))

(fn RemoveKey
  (params (InKeyToRemove :type Name))
  (bind _returnvalue (Utilities|Set|Remove (Variables|Quest|GetQuestItems) InKeyToRemove))
  (return _returnvalue))

(fn AddQuestItem)

(fn RemoveQuestItem)

(fn AddConsumable)

(fn RemoveConsumable)

(fn AddNewWeapon)

(fn RemoveWeapon)