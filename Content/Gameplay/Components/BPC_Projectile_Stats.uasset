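; Projectile stats component that loads a projectile's stats from the DT_Weapons_ProjectileStats data table.
; ConfigureStats, given a projectile name, caches its owner as BP_Projectile_Base and that actor's owner as BP_Weapon_Base, flagging itself unconfigured if either cast fails.
; It then stores the row matching that name and sets IsConfigured.
; The event graph is empty, so configuration runs only when ConfigureStats is called.
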(event EventBeginPlay)

(event EventTick
  (params (DeltaSeconds :type Float%20%28single-precision%29)))

(fn ConfigureStats
  (bind _returnvalue (Components|GetOwner))
  (if (!= (Variables|Config|GetThisProjectilename) "")
    (Utilities|FlowControl|Sequence
      (:then_0
        (bind _asbp_projectile_base (Utilities|Casting|CastToBP_Projectile_Base _returnvalue)
          (:then
            (Variables|Config|SetThisProjectile _asbp_projectile_base)
            (bind _asbp_weapon_base (Utilities|Casting|CastToBP_Weapon_Base (Components|GetOwner _returnvalue))
              (:then
                (Variables|Config|SetOwningWeapon _asbp_weapon_base))
              (:CastFailed
                (Variables|Config|SetIsConfigured false :!label _label)
                (return))))
          (:CastFailed
            (goto _label))))
      (:then_1
        (bind _returnvalue_2 (Utilities|GetDataTableRow "/Game/Data/DataTables/DT_Weapons_ProjectileStats.DT_Weapons_ProjectileStats" (Variables|Config|GetThisProjectilename))
          (:then
            (Variables|Config|SetProjectileStats _returnvalue_2)
            (Variables|Config|SetIsConfigured true)
            (return)))))))