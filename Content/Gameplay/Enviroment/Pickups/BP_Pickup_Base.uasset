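; Base pickup actor that puts a named, typed item into the player's backpack.
; A collision sphere tracks the overlapping BP_ThirdPersonCharacter and flips a readiness flag on each begin or end overlap, which drives the pickup widget's visibility.
; Interact checks readiness, passes the item to the character's BPC_Backpack component, then destroys the pickup via AfterUse and reports success.
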(event OnComponentBeginOverlap(SphereCollision)
  (params (OverlappedComponent :type Primitive%20Component%20Object%20Reference) (OtherActor :type Actor%20Object%20Reference) (OtherComp :type Primitive%20Component%20Object%20Reference) (OtherBodyIndex :type Integer) (bFromSweep :type Boolean) (SweepResult :type Hit%20Result%20Structure%20%28by%20ref%29))
  (Utilities|Casting|CastToBP_ThirdPersonCharacter OtherActor)
  (Variables|PickupConfig|SetOverlappedPlayerCharacter OtherActor)
  (PickupUpdate|UpdateIsReadytoInteract))

(event OnComponentEndOverlap(SphereCollision)
  (params (OverlappedComponent :type Primitive%20Component%20Object%20Reference) (OtherActor :type Actor%20Object%20Reference) (OtherComp :type Primitive%20Component%20Object%20Reference) (OtherBodyIndex :type Integer))
  (Utilities|Casting|CastToBP_ThirdPersonCharacter OtherActor)
  (Variables|PickupConfig|SetOverlappedPlayerCharacter 0)
  (PickupUpdate|UpdateIsReadytoInteract))

(event EventBeginPlay)

(event Collision|EventActorBeginOverlap
  (params (OtherActor :type Actor%20Object%20Reference)))

(event EventTick
  (params (DeltaSeconds :type Float%20%28single-precision%29)))

(fn ConstructionScript)

(fn UpdateIsReadytoInteract
  (Variables|PickupConfig|SetIsReadyToInteract (not (Variables|PickupConfig|GetIsReadyToInteract)))
  (PickupUpdate|UpdatePickupWidgetVisibility))

(fn UpdatePickupWidgetVisibility
  (Rendering|SetVisibility (Variables|Default|GetPickupWidget) (Variables|PickupConfig|GetIsReadyToInteract) true))

(fn AfterUse
  (Actor|DestroyActor))

(fn Interact
  (if (Variables|PickupConfig|GetIsReadyToInteract)
    (bind _overlappedplayercharacter (Variables|PickupConfig|GetOverlappedPlayerCharacter)
      (:then
        (Utilities|IsValid (Actor|GetComponentbyClass _overlappedplayercharacter "/Game/Gameplay/Components/BPC_Backpack.BPC_Backpack_C")
          (:Is%20Valid
            (Default|AddNewItem (Actor|GetComponentbyClass _overlappedplayercharacter "/Game/Gameplay/Components/BPC_Backpack.BPC_Backpack_C") (Variables|PickupConfig|GetItemName) (Variables|PickupConfig|GetItemType))
            (CallFunction|AfterUse)
            (return true))
          (:Is%20Not%20Valid
            (return false))))
      (:else
        (return false)))
    (else
      (return false))))