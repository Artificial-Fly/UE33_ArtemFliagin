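; Locked variant of a parent door that opens only once the interacting actor holds every required key.
; Interaction counts matching RequiredKeys in the actor's BPC_Character_Backpack, then either unlocks and calls the parent's door update or shows the key count on the WBP_DoorText widget.
; A light shows red when locked and green when unlocked, initialized with the hint in the Construction Script.
; A locked door with no required keys stays locked on interaction.
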(event EventBeginPlay
  (|CallParentFunction) ; This node is disabled and will not be called.\nDrag off pins to build functionality.
)

(event Collision|EventActorBeginOverlap
  (params (OtherActor :type Actor%20Object%20Reference))
  (|CallParentFunction OtherActor) ; This node is disabled and will not be called.\nDrag off pins to build functionality.
)

(event EventTick
  (params (DeltaSeconds :type Float%20%28single-precision%29))
  (|CallParentFunction DeltaSeconds) ; This node is disabled and will not be called.\nDrag off pins to build functionality.
)

(fn ConstructionScript
  (|CallParentFunction)
  (DoorUpdate|UpdateDoorLockIndicator)
  (bind _aswbp_door_text (Utilities|Casting|CastToWBP_DoorText (UserInterface|GetWidget (Variables|Default|GetDoorWidget))))
  (Default|UpdateWidgetHint _aswbp_door_text 0 (Utilities|Array|Length (Variables|DoorConfig|GetRequiredKeys))))

(fn UpdateDoorLockIndicator
  (Rendering|Components|Light|SetLightColor (Variables|Default|GetLockIndicator) (Math|Color|SelectColor "(R=1.000000,G=0.000000,B=0.006678,A=1.000000)" "(R=0.000000,G=1.000000,B=0.034225,A=1.000000)" (Variables|DoorConfig|GetIsLocked)) true))

(fn UpdateLockState
  (Variables|DoorConfig|SetIsLocked (not (Variables|DoorConfig|GetIsLocked)))
  (DoorUpdate|UpdateDoorLockIndicator))

(fn UpdateDoorState
  (if (not (Variables|DoorConfig|GetIsLocked))
    (|CallParentFunction)))

(fn InteractwithObjects
  (params (InitiatedActor :type Actor%20Object%20Reference))
  (if (not (Variables|Default|GetIsOpen))
    (Variables|Default|SetInitiatedActor InitiatedActor)
    (CallFunction|SetDoorDirection))
  (if (Variables|Default|GetIsReadyToInteract)
    (if (not (Variables|DoorConfig|GetIsLocked))
      (CallFunction|UpdateDoorState)
      (elif (Utilities|Array|IsValidIndex (Variables|DoorConfig|GetRequiredKeys))
        (bind _initiatedactor (LocalVariables|GetInitiatedActor)
          (:then
            (Utilities|IsValid (Actor|GetComponentbyClass _initiatedactor "/Game/Gameplay/Components/BPC_Character_Backpack.BPC_Character_Backpack_C")
              (:Is%20Valid
                (LocalVariables|SetL_Backpack (Actor|GetComponentbyClass _initiatedactor "/Game/Gameplay/Components/BPC_Character_Backpack.BPC_Character_Backpack_C"))
                (for _array_element (Variables|DoorConfig|GetRequiredKeys)
                  (LocalVariables|SetL_KeyName _array_element)
                  (if (Utilities|Set|Contains (Variables|/Game/Gameplay/Components/BPC_Character_Backpack.BPC_Character_Backpack_C|GetKeys (LocalVariables|GetL_Backpack)) (LocalVariables|GetL_KeyName))
                    (Math|Integer|IncrementInt (LocalVariables|GetL_KeyIncrement))))
                (if (== (LocalVariables|GetL_KeyIncrement) (Utilities|Array|Length (Variables|DoorConfig|GetRequiredKeys)))
                  (DoorUpdate|UpdateLockState)
                  (CallFunction|UpdateDoorState)
                  (else
                    ;[1 1 1] Tell player that they need keys
                    (bind _aswbp_door_text (Utilities|Casting|CastToWBP_DoorText (UserInterface|GetWidget (Variables|Default|GetDoorWidget))))
                    (Default|UpdateWidgetHint _aswbp_door_text (LocalVariables|GetL_KeyIncrement) (Utilities|Array|Length (Variables|DoorConfig|GetRequiredKeys)))
                    (return true))))
              (:Is%20Not%20Valid
                (return false))))
          (:else
            (return false)))
        (else
          (return true))))
    (else
      (return false))))