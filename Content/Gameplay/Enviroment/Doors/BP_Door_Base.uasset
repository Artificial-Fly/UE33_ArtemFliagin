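; Base interactable swinging door that pawns can open and close, with an optional open-by-default state set in the construction script.
; Box overlaps track nearby pawns and toggle interaction readiness, which drives the prompt widget's visibility and text.
; Interact picks a swing direction away from the initiator via a dot product when closed, then toggles the door if ready.
; A timeline rotates DoorRotator, playing in reverse to close and blocking re-triggering mid-swing.
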(event OnComponentBeginOverlap(BoxCollision)
  (params (OverlappedComponent :type Primitive%20Component%20Object%20Reference) (OtherActor :type Actor%20Object%20Reference) (OtherComp :type Primitive%20Component%20Object%20Reference) (OtherBodyIndex :type Integer) (bFromSweep :type Boolean) (SweepResult :type Hit%20Result%20Structure%20%28by%20ref%29))
  (bind _aspawn (Utilities|Casting|CastToPawn OtherActor))
  (Utilities|Array|Add (Variables|DoorConfig|GetOverlappedPawns) _aspawn)
  (DoorUpdate|UpdateIsReadytoInteract))

(event OnComponentEndOverlap(BoxCollision)
  (params (OverlappedComponent :type Primitive%20Component%20Object%20Reference) (OtherActor :type Actor%20Object%20Reference) (OtherComp :type Primitive%20Component%20Object%20Reference) (OtherBodyIndex :type Integer))
  (bind _aspawn (Utilities|Casting|CastToPawn OtherActor))
  (Utilities|Array|RemoveItem (Variables|DoorConfig|GetOverlappedPawns) _aspawn)
  (if (Utilities|Array|IsEmpty (Variables|DoorConfig|GetOverlappedPawns))
    (DoorUpdate|UpdateIsReadytoInteract)))

(event Custom|OpenDoor
  ;[1 1 1] Open/Close Door
  ;;[1 1 1] Check
  (if (not (Variables|DoorConfig|GetIsInProgress))
    (if (not (Variables|DoorConfig|GetIsOpen))
      (Development|PrintString "Openning the Door")
      (bind (_direction _openprogression) (Timeline|DoorTimeline PlayFromStart)
        (:Update
          ;;[1 1 1] Update
          (Variables|DoorConfig|SetIsInProgress true)
          (Transformation|SetRelativeRotation (Variables|Default|GetDoorRotator) (Math|Rotator|MakeRotator 0.0 0.0 (* (Variables|DoorConfig|GetMaxDoorAngle) (* _openprogression (Variables|Default|GetDoorOpenDirection)))) false false))
        (:Finished
          ;;[1 1 1] Finished
          (Variables|DoorConfig|SetIsInProgress false)
          (switch Utilities|FlowControl|Switch|SwitchonETimelineDirection _direction
            (:Forward
              (Variables|DoorConfig|SetIsOpen true))
            (:Backward
              (Variables|DoorConfig|SetIsOpen false))))))))

(event Custom|CloseDoor
  ;[1 1 1] Open/Close Door
  ;;[1 1 1] Check
  (if (not (Variables|DoorConfig|GetIsInProgress))
    (if (Variables|DoorConfig|GetIsOpen)
      (Development|PrintString "Closing the Door")
      (bind (_direction _openprogression) (Timeline|DoorTimeline ReverseFromEnd)
        (:Update
          ;;[1 1 1] Update
          (Variables|DoorConfig|SetIsInProgress true)
          (Transformation|SetRelativeRotation (Variables|Default|GetDoorRotator) (Math|Rotator|MakeRotator 0.0 0.0 (* (Variables|DoorConfig|GetMaxDoorAngle) (* _openprogression (Variables|Default|GetDoorOpenDirection)))) false false))
        (:Finished
          ;;[1 1 1] Finished
          (Variables|DoorConfig|SetIsInProgress false)
          (switch Utilities|FlowControl|Switch|SwitchonETimelineDirection _direction
            (:Forward
              (Variables|DoorConfig|SetIsOpen true))
            (:Backward
              (Variables|DoorConfig|SetIsOpen false))))))))

(event EventBeginPlay)

(event Collision|EventActorBeginOverlap
  (params (OtherActor :type Actor%20Object%20Reference)))

(event EventTick
  (params (DeltaSeconds :type Float%20%28single-precision%29)))

(fn ConstructionScript
  (DoorConfig|SetDoorbyDefault))

(fn UpdateIsReadytoInteract
  (Variables|DoorConfig|SetIsReadyToInteract (not (Variables|DoorConfig|GetIsReadyToInteract)))
  (DoorUpdate|UpdateDoorWidgetVisibility))

(fn UpdateDoorWidgetVisibility
  (Rendering|SetVisibility (Variables|Default|GetDoorWidget) (Variables|DoorConfig|GetIsReadyToInteract) true)
  (DoorUpdate|UpdateDoorWidgetText))

(fn SetDoorbyDefault
  (Utilities|FlowControl|Sequence
    (:then_0
      (Transformation|AddRelativeRotation (Variables|Default|GetDoorRotator) (Math|Rotator|MakeRotator 0.0 0.0 (Math|Float|SelectFloat (Variables|DoorConfig|GetMaxDoorAngle) 0.0 (Variables|DoorConfig|GetIsOpenByDefault))) false false))
    (:then_1
      (Variables|DoorConfig|SetIsOpen (Variables|DoorConfig|GetIsOpenByDefault)))))

(fn UpdateDoorWidgetText
  (bind _asw_door_text (Utilities|Casting|CastToW_DoorText (UserInterface|GetUserWidgetObject (Variables|Default|GetDoorWidget))))
  (Default|UpdateWidgetText _asw_door_text (Variables|DoorConfig|GetDoorWidgetText))
  (Default|UpdateWidgetHint _asw_door_text))

(fn UpdateDoorState
  (if (not (Variables|DoorConfig|GetIsOpen))
    (CallFunction|OpenDoor)
    (else
      (CallFunction|CloseDoor))))

(fn SetDoorDirection
  (bind _self self)
  (if (>= (Math|Vector|DotProduct (Math|Vector|GetUnitDirection(Vector) (Transformation|GetActorLocation _self) (Transformation|GetActorLocation (Variables|Default|GetInitiatedActor))) (Transformation|GetActorForwardVector _self)) 0.0)
    (Variables|Default|SetDoorOpenDirection -1.0)
    (else
      (Variables|Default|SetDoorOpenDirection 1.0))))

(fn Interact
  (params (InitiatedActor :type Actor%20Object%20Reference))
  (if (not (Variables|DoorConfig|GetIsOpen))
    (Variables|Default|SetInitiatedActor InitiatedActor)
    (CallFunction|SetDoorDirection))
  (if (Variables|DoorConfig|GetIsReadyToInteract)
    (DoorUpdate|UpdateDoorState)
    (return true)
    (else
      (return false))))