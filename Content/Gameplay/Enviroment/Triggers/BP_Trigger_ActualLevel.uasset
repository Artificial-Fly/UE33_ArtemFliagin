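; BP_Trigger_ActualLevel is an interactable level trigger that opens the current level.
; On BeginPlay it runs the parent logic, then labels its trigger widget "Current Level".
; Its Interact function casts the game instance to BP_GameInstance, calls LevelOpenActual, and returns whether the cast succeeded.
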(event EventBeginPlay
  (|CallParentFunction)
  (Variables|Default|SetTriggerWidgetText "Current Level")
  (CallFunction|UpdateTriggerWidgetText))

(event Collision|EventActorBeginOverlap
  (params (OtherActor :type Actor%20Object%20Reference))
  (|CallParentFunction OtherActor) ; This node is disabled and will not be called.\nDrag off pins to build functionality.
)

(event EventTick
  (params (DeltaSeconds :type Float%20%28single-precision%29))
  (|CallParentFunction DeltaSeconds) ; This node is disabled and will not be called.\nDrag off pins to build functionality.
)

(fn ConstructionScript
  (|CallParentFunction))

(fn Interact
  (params (InitiatedActor :type Actor%20Object%20Reference))
  (bind _asbp_game_instance (Utilities|Casting|CastToBP_GameInstance (Game|GetGameInstance))
    (:then
      (Default|LevelOpenActual _asbp_game_instance)
      (return true))
    (:CastFailed
      (return false))))