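; Save point trigger volume that saves the game when an actor overlaps it.
; It extends a parent trigger, setting the inherited widget text to "SavePoint" on BeginPlay.
; On overlap, it runs the parent logic, then calls BP_GameInstance to update level progress and save to its current data slot.
; The overlapping actor is not filtered in this Blueprint.
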(event EventBeginPlay
  (|CallParentFunction)
  (Variables|Default|SetTriggerWidgetText "SavePoint")
  (CallFunction|UpdateTriggerWidgetText))

(event Collision|EventActorBeginOverlap
  (params (OtherActor :type Actor%20Object%20Reference))
  (|CallParentFunction OtherActor)
  (bind _asbp_game_instance (Utilities|Casting|CastToBP_GameInstance (Game|GetGameInstance)))
  (Default|LevelUpdateProgress _asbp_game_instance false false false)
  (Default|GameSave _asbp_game_instance (Variables|/Game/Gameplay/BP_GameInstance.BP_GameInstance_C|GetGame_SaveData_Slot _asbp_game_instance)))

(event EventTick
  (params (DeltaSeconds :type Float%20%28single-precision%29))
  (|CallParentFunction DeltaSeconds) ; This node is disabled and will not be called.\nDrag off pins to build functionality.
)

(fn ConstructionScript
  (|CallParentFunction))