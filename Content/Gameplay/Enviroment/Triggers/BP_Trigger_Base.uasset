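; Base interactable trigger that shows a text widget while pawns overlap its box, with a stub InteractWithObjects that returns true.
; Construction sizes two boxes from one extent and lifts them to sit on the origin.
; Overlaps track pawns and toggle readiness, rather than setting it, on every entry and on the last exit, driving widget visibility.
; While ready, Tick turns the widget's scene component toward the player camera.
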(event OnComponentBeginOverlap(BoxCollision)
  (params (OverlappedComponent :type Primitive%20Component%20Object%20Reference) (OtherActor :type Actor%20Object%20Reference) (OtherComp :type Primitive%20Component%20Object%20Reference) (OtherBodyIndex :type Integer) (bFromSweep :type Boolean) (SweepResult :type Hit%20Result%20Structure%20%28by%20ref%29))
  (bind _aspawn (Utilities|Casting|CastToPawn OtherActor))
  (Utilities|Array|Add (Variables|TriggerConfig|GetOverlappedPawns) _aspawn)
  (TriggerUpdate|UpdateIsReadytoInteract))

(event OnComponentEndOverlap(BoxCollision)
  (params (OverlappedComponent :type Primitive%20Component%20Object%20Reference) (OtherActor :type Actor%20Object%20Reference) (OtherComp :type Primitive%20Component%20Object%20Reference) (OtherBodyIndex :type Integer))
  (bind _aspawn (Utilities|Casting|CastToPawn OtherActor))
  (Utilities|Array|RemoveItem (Variables|TriggerConfig|GetOverlappedPawns) _aspawn)
  (if (Utilities|Array|IsEmpty (Variables|TriggerConfig|GetOverlappedPawns))
    (TriggerUpdate|UpdateIsReadytoInteract)))

(event EventBeginPlay)

(event Collision|EventActorBeginOverlap
  (params (OtherActor :type Actor%20Object%20Reference)))

(event EventTick
  (params (DeltaSeconds :type Float%20%28single-precision%29))
  (if (Variables|TriggerConfig|GetIsReadyToInteract)
    (TriggerUpdate|UpdateTriggerTextWidgetRotation)))

(fn ConstructionScript
  (TriggerConfig|SetTriggerBoxCollision))

(fn UpdateIsReadytoInteract
  (Variables|TriggerConfig|SetIsReadyToInteract (not (Variables|TriggerConfig|GetIsReadyToInteract)))
  (TriggerUpdate|UpdateTriggerWidgetVisibility))

(fn UpdateTriggerWidgetVisibility
  (Rendering|SetVisibility (Variables|Default|GetTriggerWidget) (Variables|TriggerConfig|GetIsReadyToInteract) true))

(fn SetTriggerBoxCollision
  (Components|Box|SetBoxExtent (Variables|Default|GetBoxCollision) (Variables|TriggerConfig|GetInBoxExtent) true)
  (Transformation|SetRelativeLocation (Variables|Default|GetBoxCollision) (Math|Vector|MakeVector 0.0 0.0 (.Z (Math|Vector|BreakVector (Variables|TriggerConfig|GetInBoxExtent)))) false false)
  (Components|Box|SetBoxExtent (Variables|Default|GetBoxInteractCollision) (Variables|TriggerConfig|GetInBoxExtent) true)
  (Transformation|SetRelativeLocation (Variables|Default|GetBoxInteractCollision) (Math|Vector|MakeVector 0.0 0.0 (.Z (Math|Vector|BreakVector (Variables|TriggerConfig|GetInBoxExtent)))) false false))

(fn UpdateTriggerWidgetText
  (bind _aswbp_trigger_text (Utilities|Casting|CastToWBP_TriggerText (UserInterface|GetUserWidgetObject (Variables|Default|GetTriggerWidget))))
  (Default|UpdateWidgetText _aswbp_trigger_text (Variables|TriggerConfig|GetTriggerWidgetText)))

(fn UpdateTriggerTextWidgetRotation
  (bind _asbp_character_player (Utilities|Casting|CastToBP_Character_Player (Game|Player|GetPlayerPawn 0)))
  (LocalVariables|SetL_PlayerCameraLocation (Transformation|GetWorldLocation (Variables|/Game/Gameplay/Characters/Player/BP_Character_Player.BP_Character_Player_C|GetCamera _asbp_character_player)))
  (Transformation|SetWorldRotation (Variables|Default|GetTriggerScene) (Math|Rotator|FindLookatRotation (Transformation|GetWorldLocation (Variables|Default|GetTriggerScene)) (LocalVariables|GetL_PlayerCameraLocation)) false false))

(fn InteractwithObjects
  (params (InitiatedActor :type Actor%20Object%20Reference))
  (return true))