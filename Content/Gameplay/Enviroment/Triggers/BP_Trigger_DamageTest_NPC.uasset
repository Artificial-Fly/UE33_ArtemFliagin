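; Interactable test lever that deals damage to an assigned character, named on its trigger widget at BeginPlay.
; Interact, when ready, starts a timeline that rotates the handle mesh in a direction set by its toggle state, ignoring repeat pulls while in progress.
; When the timeline finishes, the state flips and a fixed amount of BP_Damage_Base damage is applied to the character with the lever as causer.
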(event Custom|MoveTriggerHandle
  ;[1 1 1] Move Handle
  ;;[1 1 1] Check
  (if (not (Variables|Default|GetIsInProgress))
    (bind _triggerhandleprogression (Timeline|TriggerHandleTimeline PlayFromStart)
      (:Update
        ;;[1 1 1] Update
        (Variables|Default|SetIsInProgress true)
        (TriggerUpdate|UpdateTriggerHandleAngle _triggerhandleprogression))
      (:Finished
        ;;[1 1 1] Finish
        (Variables|TriggerConfig|SetTriggerHandleState (not (Variables|TriggerConfig|GetTriggerHandleState)))
        (Variables|Default|SetIsInProgress false)
        (CallFunction|DealDamagetoSelectedCharacter)))))

(event EventBeginPlay
  (|CallParentFunction)
  (Variables|Default|SetTriggerWidgetText (Utilities|Text|FormatText "Deal Damage to {Character}" (Utilities|GetDisplayName (Variables|TriggerConfig|GetCharacterToDamage))))
  (CallFunction|UpdateTriggerWidgetText))

(event Collision|EventActorBeginOverlap
  (params (OtherActor :type Actor%20Object%20Reference))
  (|CallParentFunction OtherActor) ; This node is disabled and will not be called.\nDrag off pins to build functionality.
)

(event EventTick
  (params (DeltaSeconds :type Float%20%28single-precision%29))
  (|CallParentFunction DeltaSeconds) ; This node is disabled and will not be called.\nDrag off pins to build functionality.
)

(fn ConstructionScript
  (|CallParentFunction)
  (TriggerUpdate|UpdateTriggerHandleAngle 1.0))

(fn UpdateTriggerHandleAngle
  (params (InTimelineKoef :type Float%20%28double-precision%29))
  (if (not (Variables|TriggerConfig|GetTriggerHandleState))
    (bind _output_get (LocalVariables|SetL_TriggerHadnleDirection "0.000000,0.000000,-1.000000"))
    (LocalVariables|SetL_TriggerHandleNewAngle (* _output_get (* (Variables|TriggerConfig|GetTriggerHandleMaxAngle) InTimelineKoef)))
    (else
      (bind _output_get_2 (LocalVariables|SetL_TriggerHadnleDirection "0.000000,0.000000,1.000000"))
      (LocalVariables|SetL_TriggerHandleNewAngle (* _output_get_2 (* (Variables|TriggerConfig|GetTriggerHandleMaxAngle) InTimelineKoef)))))
  (Transformation|SetRelativeRotation (Variables|Default|GetTriggerHandleMesh) (LocalVariables|GetL_TriggerHandleNewAngle) false false))

(fn Interact
  (params (InitiatedActor :type Actor%20Object%20Reference))
  (if (Variables|Default|GetIsReadyToInteract)
    (CallFunction|MoveTriggerHandle)
    (return true)
    (else
      (return false))))

(fn DealDamagetoSelectedCharacter
  (Game|Damage|ApplyDamage (Variables|TriggerConfig|GetCharacterToDamage) 35.0 0 self "/Game/Data/Objects/BP_Damage_Base.BP_Damage_Base_C"))