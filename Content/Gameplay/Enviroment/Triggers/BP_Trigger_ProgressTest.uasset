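; BP_Trigger_ProgressTest is a trigger actor, apparently for testing progress, that the player can interact with to raise a flag.
; Interact sets IsFlagRaised and returns true only when the initiator is a BP_Character_Player, and nothing here lowers the flag again.
; Tick reapplies a green or red emissive material to the trigger mesh every frame to show the flag state.
; BeginPlay sets the trigger widget text to "E".
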(event EventBeginPlay
  (Variables|Default|SetTriggerWidgetText "E")
  (CallFunction|UpdateTriggerWidgetText))

(event Collision|EventActorBeginOverlap
  (params (OtherActor :type Actor%20Object%20Reference))
  (|CallParentFunction OtherActor) ; This node is disabled and will not be called.\nDrag off pins to build functionality.
)

(event EventTick
  (params (DeltaSeconds :type Float%20%28single-precision%29))
  (|CallParentFunction DeltaSeconds)
  (Rendering|Material|SetMaterial (Variables|Default|GetTriggermesh) 0 (select (Variables|Default|GetIsFlagRaised) "/Game/Materials/Colors/MI_Emissive_Green.MI_Emissive_Green" "/Game/Materials/Colors/MI_Emissive_Red.MI_Emissive_Red")))

(fn ConstructionScript
  (|CallParentFunction))

(fn Interact
  (params (InitiatedActor :type Actor%20Object%20Reference))
  (Utilities|Casting|CastToBP_Character_Player InitiatedActor
    (:then
      (Variables|Default|SetIsFlagRaised true)
      (return true))
    (:CastFailed
      (return false))))